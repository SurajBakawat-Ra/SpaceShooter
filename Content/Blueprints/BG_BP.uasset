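; BG_BP is an actor, likely a background piece going by its name, that moves continuously along X at a fixed height.
; A timeline starts on BeginPlay and lerps the actor's location between two hard-coded world positions without sweeping.
; Each time the timeline finishes, the Rev flag toggles and selects either ResetMap to play in reverse or BegMap to play from the start.
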(event Custom|ResetMap
  (bind _newtrack_0 (Timeline|Timeline_0 Reverse)
    (:Update
      (Transformation|SetActorLocation (Math|Vector|Lerp(Vector) "3000.000000, 0,-300.000000" "-2800.000000, 0,-300.000000" _newtrack_0) false false))
    (:Finished
      (if (Variables|Default|GetRev)
        (CallFunction|ResetMap)
        (Variables|Default|SetRev false)
        (else
          (CallFunction|BegMap)
          (Variables|Default|SetRev true))))))

(event Custom|BegMap
  (bind _newtrack_0 (Timeline|Timeline_0 PlayFromStart)
    (:Update
      (Transformation|SetActorLocation (Math|Vector|Lerp(Vector) "3000.000000, 0,-300.000000" "-2800.000000, 0,-300.000000" _newtrack_0) false false))
    (:Finished
      (if (Variables|Default|GetRev)
        (CallFunction|ResetMap)
        (Variables|Default|SetRev false)
        (else
          (CallFunction|BegMap)
          (Variables|Default|SetRev true))))))

(event EventBeginPlay
  (bind _newtrack_0 (Timeline|Timeline_0 Play)
    (:Update
      (Transformation|SetActorLocation (Math|Vector|Lerp(Vector) "3000.000000, 0,-300.000000" "-2800.000000, 0,-300.000000" _newtrack_0) false false))
    (:Finished
      (if (Variables|Default|GetRev)
        (CallFunction|ResetMap)
        (Variables|Default|SetRev false)
        (else
          (CallFunction|BegMap)
          (Variables|Default|SetRev true))))))

(event Collision|EventActorBeginOverlap
  (params (OtherActor :type Actor%20Object%20Reference)))

(fn ConstructionScript)