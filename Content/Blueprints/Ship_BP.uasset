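; Ship Blueprint that turns touch swipes into actions: right and left call ShootRight and ShootLeft, up calls Teleport, and down only prints.
; Two touch input actions share the pressed state and start position, both read from Touch1.
; While pressed, Tick waits for over 100 units of movement, then classifies the swipe by dominant axis.
; Two duplicate DoOnce paths do this, each reset by its own action's release.
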(event EventBeginPlay)

(event Collision|EventActorBeginOverlap
  (params (OtherActor :type Actor%20Object%20Reference)))

(event EventTick
  (params (DeltaSeconds :type Float%20%28single-precision%29))
  (bind _returnvalue (Game|GetPlayerController 0))
  (bind _returnvalue_2 (Game|GetPlayerController 0))
  (bind (_locationx _locationy) (Class|PlayerController|GetInputTouchState _returnvalue_2 "Touch1"))
  (bind (_locationx_2 _locationy_2) (Class|PlayerController|GetInputTouchState _returnvalue "Touch1"))
  (bind _returnvalue_3 (Math|Vector2D|MakeVector2D _locationx_2 _locationy_2))
  (bind _returnvalue_4 (Math|Vector2D|MakeVector2D _locationx _locationy))
  (Utilities|FlowControl|Sequence
    (:then_0
      (if (Variables|Default|GetIsPressed)
        (if (> (Math|Vector2D|Vector2DLength (- (Variables|Default|GetTouchStart2DVector) _returnvalue_4)) 1e+02)
          (Utilities|FlowControl|DoOnce false
            (:Completed
              (Variables|Default|SetTouchEnd2DVector _returnvalue_4)
              (if (> (Math|Float|Absolute(Float) (.X (Math|Vector2D|BreakVector2D (- (Variables|Default|GetTouchEnd2DVector) (Variables|Default|GetTouchStart2DVector))))) (Math|Float|Absolute(Float) (.Y (Math|Vector2D|BreakVector2D (- (Variables|Default|GetTouchEnd2DVector) (Variables|Default|GetTouchStart2DVector))))))
                (if (> (.X (Math|Vector2D|BreakVector2D (- (Variables|Default|GetTouchEnd2DVector) (Variables|Default|GetTouchStart2DVector)))) 0.0)
                  (Development|PrintString "Right")
                  (Class|ShipController|ShootRight)
                  (else
                    (Development|PrintString "Left")
                    (Class|ShipController|ShootLeft)))
                (elif (> (.Y (Math|Vector2D|BreakVector2D (- (Variables|Default|GetTouchEnd2DVector) (Variables|Default|GetTouchStart2DVector)))) 0.0)
                  (Development|PrintString "Down")
                  (else
                    (Development|PrintString "Up")
                    (Class|ShipController|Teleport)))))))))
    (:then_1
      (if (Variables|Default|GetIsPressed)
        (if (> (Math|Vector2D|Vector2DLength (- (Variables|Default|GetTouchStart2DVector) _returnvalue_3)) 1e+02)
          (Utilities|FlowControl|DoOnce false
            (:Completed
              (Variables|Default|SetTouchEnd2DVector _returnvalue_3)
              (if (> (Math|Float|Absolute(Float) (.X (Math|Vector2D|BreakVector2D (- (Variables|Default|GetTouchEnd2DVector) (Variables|Default|GetTouchStart2DVector))))) (Math|Float|Absolute(Float) (.Y (Math|Vector2D|BreakVector2D (- (Variables|Default|GetTouchEnd2DVector) (Variables|Default|GetTouchStart2DVector))))))
                (if (> (.X (Math|Vector2D|BreakVector2D (- (Variables|Default|GetTouchEnd2DVector) (Variables|Default|GetTouchStart2DVector)))) 0.0)
                  (Development|PrintString "Right")
                  (Class|ShipController|ShootRight)
                  (else
                    (Development|PrintString "Left")
                    (Class|ShipController|ShootLeft)))
                (elif (> (.Y (Math|Vector2D|BreakVector2D (- (Variables|Default|GetTouchEnd2DVector) (Variables|Default|GetTouchStart2DVector)))) 0.0)
                  (Development|PrintString "Down")
                  (else
                    (Development|PrintString "Up")
                    (Class|ShipController|Teleport)))))))))))

(event Input|ActionEvents|InputActionTouchStart2
  (params (Key :type Key%20Structure))
  (bind _returnvalue (Game|GetPlayerController 0))
  (bind (_locationx _locationy) (Class|PlayerController|GetInputTouchState _returnvalue "Touch1"))
  (bind _returnvalue_2 (Math|Vector2D|MakeVector2D _locationx _locationy))
  (:Pressed
    (Variables|Default|SetIsPressed true)
    (Variables|Default|SetTouchStart2DVector _returnvalue_2))
  (:Released
    (Variables|Default|SetIsPressed false)
    (Utilities|FlowControl|DoOnce false) ; enters at Reset
  ))

(event Input|ActionEvents|InputActionTouchStart
  (params (Key :type Key%20Structure))
  (bind _returnvalue (Game|GetPlayerController 0))
  (bind (_locationx _locationy) (Class|PlayerController|GetInputTouchState _returnvalue "Touch1"))
  (bind _returnvalue_2 (Math|Vector2D|MakeVector2D _locationx _locationy))
  (:Pressed
    (Variables|Default|SetIsPressed true)
    (Variables|Default|SetTouchStart2DVector _returnvalue_2))
  (:Released
    (Variables|Default|SetIsPressed false)
    (Utilities|FlowControl|DoOnce false) ; enters at Reset
  ))

(fn ConstructionScript)